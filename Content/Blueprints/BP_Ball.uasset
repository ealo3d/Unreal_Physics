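; BP_Ball is a player-controlled physics ball driven through Enhanced Input.
; BeginPlay adds the default mapping context after a short delay.
; Look input rotates the controller's pitch and yaw.
; Move input applies forces to the Sphere component along forward and right vectors built from control yaw only, so rolling follows the view direction horizontally.
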(event Input|EnhancedActionEvents|EnhancedInputActionIA_Move
  (params (ActionValue :type Vector%202D%20Structure) (ElapsedSeconds :type Float%20%28double-precision%29) (TriggeredSeconds :type Float%20%28double-precision%29) (InputAction :type Input%20Action%20Object%20Reference :default "/Game/Input/Actions/IA_Move.IA_Move"))
  (bind _returnvalue (Pawn|GetControlRotation :!class /Script/Engine.Pawn))
  (bind _sphere (Variables|Default|GetSphere))
  (bind _returnvalue_2 (Math|Rotator|MakeRotator 0.0 0.0 (.yaw _returnvalue)))
  (Physics|AddForce _sphere (* (Math|Vector|GetForwardVector _returnvalue_2) (.y ActionValue) 5e+04) "None" false)
  (Physics|AddForce _sphere (* (Math|Vector|GetRightVector _returnvalue_2) (.x ActionValue) 5e+04) "None" false))

(event Input|EnhancedActionEvents|EnhancedInputActionIA_Look
  (params (ActionValue :type Vector%202D%20Structure) (ElapsedSeconds :type Float%20%28double-precision%29) (TriggeredSeconds :type Float%20%28double-precision%29) (InputAction :type Input%20Action%20Object%20Reference :default "/Game/Input/Actions/IA_Look.IA_Look"))
  (Pawn|Input|AddControllerPitchInput (.y ActionValue))
  (Pawn|Input|AddControllerYawInput (.x ActionValue)))

(event EventBeginPlay
  (Utilities|FlowControl|Delay 0.2)
  (Input|AddMappingContext (PlayerController|LocalPlayerSubsystems|GetEnhancedInputLocalPlayerSubsystem (Game|GetPlayerController 0)) "/Game/Input/IMC_Default.IMC_Default" 0 "(bIgnoreAllPressedKeysUntilRelease=True,bForceImmediately=False,bNotifyUserSettings=False)"))

(fn ConstructionScript)